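; BP_CustomController is a custom controller that manages Enhanced Input mapping contexts for gameplay phases.
; On BeginPlay it binds an event to BP_CustomGameMode's gameplay phase change, then calls NewGamePlayPhase on that game mode.
; ChangeMappingContext switches on game state, clearing every active context listed in AllMappingContext before adding the new one.
; Only the Gogles state is handled, mapping to IMC_JumelleGame.
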(event EventBeginPlay
  (bind _asbp_custom_game_mode (Utilities|Casting|CastToBP_CustomGameMode (Game|GetGameMode)))
  (EventDispatchers|BindEventtoChangeGameplayPhase _asbp_custom_game_mode (EventDispatchers|CreateEvent :!event ChangeMappingContext))
  (Default|NewGamePlayPhase _asbp_custom_game_mode))

(fn ConstructionScript)

(fn ChangeMappingContext
  (params (gameState :type E_gameState%20Enum :default "NewEnumerator0"))
  (switch Utilities|FlowControl|Switch|SwitchonE_gameState gameState
    (:NewEnumerator0
      (CallFunction|RemoveMappingContext)
      (Input|AddMappingContext (PlayerController|LocalPlayerSubsystems|GetEnhancedInputLocalPlayerSubsystem) "/Game/game/JumelleGame/inputs/IMC_JumelleGame.IMC_JumelleGame" 0 "(bIgnoreAllPressedKeysUntilRelease=True,bForceImmediately=False,bNotifyUserSettings=False)"))))

(fn RemoveMappingContext
  (bind _returnvalue (PlayerController|LocalPlayerSubsystems|GetEnhancedInputLocalPlayerSubsystem))
  (for _array_element (LocalVariables|GetallMappingContext)
    (if (.ReturnValue (Class|EnhancedInputSubsystemInterface|HasMappingContext _returnvalue _array_element))
      (Input|RemoveMappingContext _returnvalue _array_element "(bIgnoreAllPressedKeysUntilRelease=True,bForceImmediately=False,bNotifyUserSettings=False)"))))